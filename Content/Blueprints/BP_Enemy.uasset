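; BP_Enemy is an enemy actor that is destroyed when the third-person player character overlaps its Collision component.
; The overlap sets Health to a negative value rather than destroying the actor directly.
; CheckHealth starts on BeginPlay and re-calls itself after a short Delay, polling Health without Tick and destroying the actor once it drops below zero.
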(event OnComponentBeginOverlap(Collision)
  (params (OverlappedComponent :type Primitive%20Component%20Object%20Reference) (OtherActor :type Actor%20Object%20Reference) (OtherComp :type Primitive%20Component%20Object%20Reference) (OtherBodyIndex :type Integer) (bFromSweep :type Boolean) (SweepResult :type Hit%20Result%20Structure%20%28by%20ref%29))
  (Utilities|Casting|CastToBP_ThirdPersonCharacter OtherActor)
  (Variables|Default|SetHealth -1.0))

(event Custom|Check%20Health
  (Utilities|FlowControl|Delay 0.1)
  (if (>= (Variables|Default|GetHealth) 0.0)
    (CallFunction|CheckHealth)
    (else
      (Actor|DestroyActor))))

(event EventBeginPlay
  (CallFunction|CheckHealth))

(event Collision|EventActorBeginOverlap
  (params (OtherActor :type Actor%20Object%20Reference)))

(event EventTick
  (params (DeltaSeconds :type Float%20%28single-precision%29)))

(fn ConstructionScript)