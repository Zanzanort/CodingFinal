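; BP_EnemySpawner spawns waves of BP_Enemy at BP_EnemySpawn markers in the level, starting a new wave once no enemies remain.
; BeginPlay gathers and prints the spawn location count, then SpawnEnemies gives each location a coin-flip chance to spawn.
; CheckEnemyCount re-calls itself, after a short delay while enemies exist or immediately after triggering a new wave, instead of using Tick.
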(event Custom|SpawnEnemies
  (for _array_element (stale EventBeginPlay _outactors)
    (if (Math|Random|RandomBool)
      (Game|SpawnActorfromClass "/Game/Blueprints/BP_Enemy.BP_Enemy_C" (Transformation|GetActorTransform _array_element) "Undefined" "MultiplyWithRoot" 0 0))))

(event Custom|CheckEnemyCount
  (bind _outactors (Actor|GetAllActorsOfClass "/Game/Blueprints/BP_Enemy.BP_Enemy_C"))
  (if (> (Utilities|Array|Length _outactors) 0)
    (Utilities|FlowControl|Delay 2.0)
    (CallFunction|CheckEnemyCount)
    (else
      (CallFunction|SpawnEnemies)
      (CallFunction|CheckEnemyCount))))

(event EventBeginPlay
  (bind _outactors (Actor|GetAllActorsOfClass "/Game/Blueprints/BP_EnemySpawn.BP_EnemySpawn_C"))
  (Development|PrintString (Utilities|String|Append "There Are " (Utilities|String|ToString(Integer) (Utilities|Array|Length _outactors)) " Spawn Locations"))
  (CallFunction|SpawnEnemies)
  (CallFunction|CheckEnemyCount))

(event Collision|EventActorBeginOverlap
  (params (OtherActor :type Actor%20Object%20Reference)))

(event EventTick
  (params (DeltaSeconds :type Float%20%28single-precision%29)))

(fn ConstructionScript)