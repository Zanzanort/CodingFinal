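; BP_CoolBox is a spawner actor that endlessly produces BP_Key actors above its Cube component.
; On BeginPlay it prints debug messages showing its name and the spawn point, offset upward from the cube.
; It then spawns a key immediately and repeats through a Delay that loops back on itself, paced by SpawnDelay, with no stop condition.
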(event EventBeginPlay
  (bind _cube (Variables|Default|GetCube))
  (bind _returnvalue (Transformation|GetWorldLocation _cube))
  (bind _returnvalue_2 (+ _returnvalue "0.000000,0.000000,200.000000"))
  (Development|PrintString (Utilities|String|Append (Utilities|GetDisplayName self) " Exists")) ; Similar to cout/print. Sends text.
  (Development|PrintString (Utilities|String|ToString(Vector) _returnvalue_2) true true "(R=1.000000,G=0.080133,B=0.000000,A=1.000000)" 1e+01)
  (Game|SpawnActorfromClass "/Game/Blueprints/BP_Key.BP_Key_C" (Math|Transform|MakeTransform _returnvalue_2 "0, 0, 0" "1.000000,1.000000,1.000000") "Undefined" "MultiplyWithRoot" 0 0 :!label _label)
  (Utilities|FlowControl|Delay (Variables|Default|GetSpawnDelay))
  (goto _label))

(event Collision|EventActorBeginOverlap
  (params (OtherActor :type Actor%20Object%20Reference)))

(event EventTick
  (params (DeltaSeconds :type Float%20%28single-precision%29)))

(fn ConstructionScript)