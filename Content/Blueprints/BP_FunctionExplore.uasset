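; Function practice Blueprint that prints color-coded messages when play begins.
; BeginPlay colors each entry in Names by length through GetColorByLength, then colors sums of random integer pairs by sign through Add2N.
; Both feed the Say event, which swaps one specific orange for a random color, though neither function outputs that orange.
; GetColorByLength's grayscale branch is unreachable because its length >= 0 check always passes.
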(event Custom|Say
  (params (InString :type String) (TextColor :type Linear%20Color%20Structure :default "(R=1.000000,G=0.737225,B=0.287390,A=1.000000)"))
  ;[1 1 1] Comment
  (if (== TextColor "(R=1.000000,G=0.737910,B=0.287441,A=1.000000)")
    (Development|PrintString InString true true (Utilities|Struct|MakeLinearColor (Math|Random|RandomFloat) (Math|Random|RandomFloat) (Math|Random|RandomFloat) 1.0) 1e+02)
    (else
      (Development|PrintString InString true true TextColor 1e+02))))

(event EventBeginPlay
  ;[1 1 1] Comment
  (Development|PrintString "Exploring..." true true "(R=0.000000,G=0.660000,B=1.000000,A=1.000000)" 5.0)
  ;[1 1 1] Comment
  (for _array_element (Variables|Default|GetNames)
    (bind _clrreturn (CallFunction|GetColorbyLength _array_element))
    (CallFunction|Say _array_element _clrreturn))
  ;[1 1 1] Comment
  (for _index (range 0 10)
    (bind (_colorout _z) (CallFunction|Add2N (Math|Random|RandomIntegerinRange -10 10) (Math|Random|RandomIntegerinRange -10 10)))
    (CallFunction|Say (Utilities|String|ToString(Integer) _z) _colorout)))

(event Collision|EventActorBeginOverlap
  (params (OtherActor :type Actor%20Object%20Reference)))

(event EventTick
  (params (DeltaSeconds :type Float%20%28single-precision%29)))

(fn ConstructionScript)

(fn GetColorbyLength
  (params (strInput :type String))
  (bind _returnvalue (Utilities|String|Len strInput))
  (bind _returnvalue_2 (- _returnvalue 5))
  (bind _returnvalue_3 (* _returnvalue_2 0.2))
  (if (<= _returnvalue 5)
    (LocalVariables|SetoutputColor "(R=0.869924,G=0.000000,B=1.000000,A=1.000000)")
    (elif (>= _returnvalue 0)
      (LocalVariables|SetoutputColor "(R=1.000000,G=0.039222,B=0.000000,A=1.000000)")
      (else
        (LocalVariables|SetoutputColor (Utilities|Struct|MakeLinearColor _returnvalue_3 _returnvalue_3 _returnvalue_3 1.0)))))
  (return (LocalVariables|GetoutputColor)))

(fn Add2N
  (params (x :type Integer) (y :type Integer))
  (bind _returnvalue (+ x y))
  (if (< _returnvalue 0)
    (LocalVariables|SetColor "(R=1.000000,G=0.041135,B=0.000000,A=1.000000)")
    (else
      (LocalVariables|SetColor "(R=0.101396,G=1.000000,B=0.000000,A=1.000000)")))
  (return (LocalVariables|GetColor) _returnvalue))